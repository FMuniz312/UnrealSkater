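; BP_ParentTrigger is a trigger Blueprint, named as a parent class, that labels itself with a text component.
; Its construction script sets TRTriggerName to the TriggerName text, or, when that is empty, to the object's name to the left of the "_C_" suffix.
; It also forces the label's world scale to one, so the text stays the same size regardless of the actor's scale.
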(fn `UserConstructionScript`
  (bind _trtriggername (`self.TRTriggerName`))
  (`/Engine/EditorBlueprintResources/StandardMacros.IsValid` _trtriggername
    (:`Is Valid`
      (`TextRenderComponent.K2_SetText` _trtriggername (select `bool` (`KismetTextLibrary.TextIsEmpty` (`self.TriggerName`)) :`false` (`self.TriggerName`) :`true` (`KismetTextLibrary.Conv_StringToText` (`KismetStringLibrary.Split` (`KismetSystemLibrary.GetObjectName` self) "_C_"))))
      (`SceneComponent.SetWorldScale3D` _trtriggername (1.0 1.0 1.0)))))