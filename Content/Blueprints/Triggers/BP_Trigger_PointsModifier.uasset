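; Trigger volume that adds or removes points, depending on its AddPoints setting, when a jumping skater overlaps its box.
; Jump state comes from the actor's gameplay tags, and points go to its AC_PointsSystem component.
; High skater speed grants bonus points on additions and briefly fires a random spark effect at the right foot.
; Awarding points also plays a trick sound and an optional cutscene sequence.
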(event `self.Box.OnComponentBeginOverlap`
  (params (OverlappedComponent :type "PrimitiveComponent Object Reference") (OtherActor :type "Actor Object Reference") (OtherComp :type "PrimitiveComponent Object Reference") (OtherBodyIndex :type Integer) (bFromSweep :type Boolean) (SweepResult :type "HitResult Structure (by ref)"))
  (bind _p_sparks_e (`self.P_Sparks_E`))
  (bind _asbpi_gameplay_tag_user (cast `/Game/Interfaces/BPI_GameplayTagUser` OtherActor))
  (bind _container (`/Game/Interfaces/BPI_GameplayTagUser.GetTagsContainer` _asbpi_gameplay_tag_user))
  (if (`BlueprintGameplayTagLibrary.HasTag` _container (struct :`TagName` "Character.Actions.Jumping") true)
    (set `self.currenttarget` (`self.GetComponentByClass` OtherActor "/Game/ActorComponents/AC_PointsSystem.AC_PointsSystem_C"))
    (`|ExecutionSequence`
      (:`then_0`
        (bind _asbpi_abpskater (cast `/Game/Interfaces/BPI_ABPSkater` OtherActor))
        (bind _percentage (`/Game/Interfaces/BPI_ABPSkater.GetSpeedPercentage` _asbpi_abpskater))
        (if (> _percentage 80.0)
          (set `self.bonusPoints` 5.0)
          (bind (_leftfoot _rightfoot) (`/Game/Interfaces/BPI_ABPSkater.GetIKFootEffectors` _asbpi_abpskater))
          (`ParticleSystemComponent.SetTemplate` _p_sparks_e (`KismetArrayLibrary.Array_Random` (`|MakeArray` "/Game/Realistic_Starter_VFX_Pack_Vol2/Particles/Sparks/P_Sparks_A.P_Sparks_A" "/Game/Realistic_Starter_VFX_Pack_Vol2/Particles/Sparks/P_Sparks_B.P_Sparks_B" "/Game/Realistic_Starter_VFX_Pack_Vol2/Particles/Sparks/P_Sparks_C.P_Sparks_C" "/Game/Realistic_Starter_VFX_Pack_Vol2/Particles/Sparks/P_Sparks_D.P_Sparks_D" "/Game/Realistic_Starter_VFX_Pack_Vol2/Particles/Sparks/P_Sparks_E.P_Sparks_E" :!type "ParticleSystem Object Reference")))
          (`SceneComponent.K2_SetWorldLocation` _p_sparks_e _rightfoot false false)
          (`ActorComponent.Activate` _p_sparks_e true)
          (`KismetSystemLibrary.Delay` 1.0)
          (`ActorComponent.Deactivate` _p_sparks_e)
          (else
            (set `self.bonusPoints` 0.0))))
      (:`then_1`
        (`/Engine/EditorBlueprintResources/StandardMacros.IsValid` (`self.currenttarget`)
          (:`Is Valid`
            (if (`self.AddPoints`)
              (`/Game/ActorComponents/AC_PointsSystem.AddPoints` (`self.currenttarget`) (+ (`self.PointsToUpdate`) (`self.bonusPoints`)))
              (`GameplayStatics.PlaySound2D` "/Game/Sound/SFX/tony-hawk-special-trick-sound-effect_CpjaBfU.tony-hawk-special-trick-sound-effect_CpjaBfU" 0.5 1.0 0.0 null null)
              (bind _cutscene (`self.Cutscene`)
                (:`then`
                  (`MovieSceneSequencePlayer.Play` (`LevelSequenceActor.SequencePlayer` _cutscene)))
                (:`else`))
              (else
                (`/Game/ActorComponents/AC_PointsSystem.RemovePoints` (`self.currenttarget`) (`self.PointsToUpdate`)))))))
      (:`then_2`
        (set `self.currenttarget` null)))))

(fn `UserConstructionScript`
  (`parent.UserConstructionScript`))