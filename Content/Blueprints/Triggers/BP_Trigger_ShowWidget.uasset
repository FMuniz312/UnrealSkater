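; BP_Trigger_ShowWidget is a box trigger that updates a tutorial message or the welcome sign on the skater HUD.
; On overlap, it checks the actor's tags through BPI_GameplayTagUser and adds TagToUpdate if missing, so each tag fires only once per holder.
; A switch on that tag routes the Welcome Sign tag to UpdateWelcomeSign and all others to UpdateTutorialState with configurable text and duration.
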(event `self.Box.OnComponentBeginOverlap`
  (params (OverlappedComponent :type "PrimitiveComponent Object Reference") (OtherActor :type "Actor Object Reference") (OtherComp :type "PrimitiveComponent Object Reference") (OtherBodyIndex :type Integer) (bFromSweep :type Boolean) (SweepResult :type "HitResult Structure (by ref)"))
  (bind _asbpi_gameplay_tag_user (cast `/Game/Interfaces/BPI_GameplayTagUser` OtherActor))
  (bind _container (`/Game/Interfaces/BPI_GameplayTagUser.GetTagsContainer` _asbpi_gameplay_tag_user))
  (if (not (`BlueprintGameplayTagLibrary.HasTag` _container (`self.tagToUpdate`) true))
    (`/Game/Interfaces/BPI_GameplayTagUser.AddNewTags` _asbpi_gameplay_tag_user (`BlueprintGameplayTagLibrary.MakeGameplayTagContainerFromTag` (`self.tagToUpdate`)))
    (`|SwitchGameplayTag` (`self.tagToUpdate`)
      (:`Default`
        (bind _ashud_skater (cast `/Game/Blueprints/HUD_Skater` (`PlayerController.GetHUD` (`GameplayStatics.GetPlayerController` 0))))
        (`/Game/UI/Widgets/WB_GameplayHUD.UpdateTutorialState` (`/Game/Blueprints/HUD_Skater.WB_GameplayHUD` _ashud_skater) (`self.showUI`) (`self.tutorialMessageDuration`) (`self.Tutorial Text`)))
      (:`PlayerState.TurorialsSeen.WelcomeSign`
        (bind _ashud_skater_2 (cast `/Game/Blueprints/HUD_Skater` (`PlayerController.GetHUD` (`GameplayStatics.GetPlayerController` 0))))
        (`/Game/UI/Widgets/WB_GameplayHUD.UpdateWelcomeSign` (`/Game/Blueprints/HUD_Skater.WB_GameplayHUD` _ashud_skater_2) (`self.showUI`))))))

(fn `UserConstructionScript`
  (`parent.UserConstructionScript`))