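; Actor component that tracks a current points value against a configurable maximum, with functions to add, remove, set, reset and read points.
; AddPoints and SetPoints clamp between zero and MaxPoints, while RemovePoints clamps its result to a fixed 0–1 range instead.
; Add and remove broadcast OnPointsUpdated with a direction flag and the amount actually changed.
; Setting, resetting and changing the maximum broadcast nothing, and a new maximum leaves current points untouched.
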(fn `AddPoints`
  (params (valueToAdd :type "Float (double-precision)"))
  (locals (finalValue :type "Float (double-precision)" :default 0.0) (addedValue :type "Float (double-precision)"))
  (set `local.finalValue` (`KismetMathLibrary.FClamp` (+ (`self.CurrentPoints`) (`KismetMathLibrary.Abs` valueToAdd)) 0.0 (`self.MaxPoints`)))
  (set `local.addedValue` (- (`local.finalValue`) (`self.CurrentPoints`)))
  (set `self.CurrentPoints` (`local.finalValue`))
  (`self.OnPointsUpdated` true (`local.addedValue`)))

(fn `GetPoints`
  (returns (CurrentPoints :type "Float (double-precision)") (MaxPoints :type "Float (double-precision)"))
  (return (`self.CurrentPoints`) (`self.MaxPoints`)))

(fn `RemovePoints`
  (params (valueToRemove :type "Float (double-precision)"))
  (locals (finalValue :type "Float (double-precision)") (removedValue :type "Float (double-precision)"))
  (set `local.finalValue` (`KismetMathLibrary.FClamp` (- (`self.CurrentPoints`) (`KismetMathLibrary.Abs` valueToRemove))))
  (set `local.removedValue` (- (`self.CurrentPoints`) (`local.finalValue`)))
  (set `self.CurrentPoints` (`local.finalValue`))
  (`self.OnPointsUpdated` false (`local.removedValue`)))

(fn `ResetPoints`
  (set `self.CurrentPoints` 0.0))

(fn `SetNewMaxPoints`
  (params (MaxPoints :type "Float (double-precision)"))
  (set `self.MaxPoints` MaxPoints))

(fn `SetPoints`
  (params (CurrentPoints :type "Float (double-precision)"))
  (set `self.CurrentPoints` (`KismetMathLibrary.FClamp` CurrentPoints 0.0 (`self.MaxPoints`))))